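; Game mode for a number-baseball guessing game that scores client guesses against a target number.
; It tracks player controllers on login and logout, storing each one's array index as PlayerOrder on the player state.
; Validated messages are compared with the joined Score digits via CheckScore, producing Strike, Ball and Out counts.
; Results, game over at three strikes and restart are only printed, with no state reset.
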(event `self.K2_PostLogin`
  (params (NewPlayer :type "PlayerController Object Reference"))
  (bind _asbp_base_ball_player_controller (cast `/Game/Network/Blueprint/BP_BaseBallPlayerController` NewPlayer))
  (bind _returnvalue (`KismetArrayLibrary.Array_Add` (`self.All_PCs`) _asbp_base_ball_player_controller))
  (bind _asbp_base_ball_game_player_state (cast `/Game/Network/Blueprint/BP_BaseBallGamePlayerState` (`GameplayStatics.GetPlayerState` _returnvalue)))
  (set `/Game/Network/Blueprint/BP_BaseBallGamePlayerState.PlayerOrder` _returnvalue _asbp_base_ball_game_player_state))

(event `self.K2_OnLogout`
  (params (ExitingController :type "Controller Object Reference"))
  (bind _asbp_base_ball_player_controller (cast `/Game/Network/Blueprint/BP_BaseBallPlayerController` ExitingController))
  (`KismetArrayLibrary.Array_RemoveItem` (`self.All_PCs`) _asbp_base_ball_player_controller))

(event `GotMessageFromClient`
  (params (Msg :type String) (PlayerState :type "/Game/Network/Blueprint/BP_BaseBallGamePlayerState Object Reference"))
  (bind _goalscore (`self.GoalScore`))
  (bind _output_get (set `self.Msg` Msg))
  (bind _returnvalue (`BaseBallCheck.CheckString` _output_get))
  (if _returnvalue
    (`|ExecutionSequence`
      (:`then_0`
        (set `self.GoalScore` "")
        (for _array_element (`self.Score`)
          (set `self.GoalScore` (`KismetStringLibrary.Concat_StrStr` (`self.GoalScore`) (`KismetStringLibrary.Conv_IntToString` _array_element))))
        (`KismetSystemLibrary.PrintString` _goalscore)
        (bind _returnvalue_2 (`BaseBallCheck.CheckScore` _goalscore (`self.Msg`)))
        (bind _output_get_2 (set `self.Result` _returnvalue_2))
        (bind (_strike _ball _out) (break `BaseBallResult` _output_get_2))
        (for (_array_element_2 _array_index) (`|MakeArray` _strike _ball _out)
          (`|ExecutionSequence`
            (:`then_0`
              (if (== _array_index 0)
                (`KismetSystemLibrary.PrintString` (`KismetStringLibrary.Concat_StrStr` (`KismetStringLibrary.Conv_IntToString` _array_element_2) " Strikes!"))
                (if (== _array_element_2 3)
                  (`KismetSystemLibrary.PrintString` "Game Over!"))))
            (:`then_1`
              (if (== _array_index 1)
                (`KismetSystemLibrary.PrintString` (`KismetStringLibrary.Concat_StrStr` (`KismetStringLibrary.Conv_IntToString` _array_element_2) " Ball!"))))
            (:`then_2`
              (if (== _array_index 2)
                (`KismetSystemLibrary.PrintString` (`KismetStringLibrary.Concat_StrStr` (`KismetStringLibrary.Conv_IntToString` _array_element_2) " Out!"))))))))))

(event `RestartGame`
  (`KismetSystemLibrary.PrintString` "Restart Game!!!" true true (struct :`G` 0.66 :`B` 1.0 :`A` 1.0) 5.0))

(fn `UserConstructionScript`)