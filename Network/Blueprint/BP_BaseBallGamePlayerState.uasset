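; BP_BaseBallGamePlayerState is the baseball game's player state Blueprint, currently holding only debug logging.
; On BeginPlay it finds every BP_BaseBallPlayerController and prints each one's name and array index in long-lasting red text.
; An unconnected chain would print PlayerOrder on both authority and remote when the owning controller is local, but it never runs.
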(event `self.ReceiveBeginPlay`
  (bind _outactors (`GameplayStatics.GetAllActorsOfClass` "/Game/Network/Blueprint/BP_BaseBallPlayerController.BP_BaseBallPlayerController_C"))
  (for (_array_element _array_index) _outactors
    (`KismetSystemLibrary.PrintString` (`KismetStringLibrary.Concat_StrStr` (`KismetSystemLibrary.GetDisplayName` _array_element) "  !!! Number !!! :" (`KismetStringLibrary.Conv_IntToString` _array_index)) true true (struct :`R` 1.0 :`B` 0.065753 :`A` 1.0) 250.0)))

(fn `UserConstructionScript`)