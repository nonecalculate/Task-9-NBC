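; BP_PC_Chat is the player controller for a networked chat game, creating the chat panel for the local player and focusing its input on Enter.
; SR_SubmitChat loops over the GameState's PlayerArray, pushing each message to every controller's panel through OC_UpdateChat.
; The same loop calls TGM_CheckGoal on each controller, so BP_GM_Chat's GetMessage receives the message once per player for goal checking.
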(event `self.ReceiveBeginPlay`
  (if (`self.IsLocalPlayerController`)
    (bind _returnvalue (`|CreateWidget` "/Game/Network/0325/Widget/WB_ChatPanel.WB_ChatPanel_C" self))
    (bind _output_get (set `self.WB_ChatPanel` _returnvalue))
    (`UserWidget.AddToViewport` _output_get 0)))

(event `Key|Enter`
  (params (Key :type "Key Structure"))
  (:`Pressed`
    (bind _wb_chatpanel (`self.WB_ChatPanel`)
      (:`then`
        (`Widget.SetKeyboardFocus` (`/Game/Network/0325/Widget/WB_ChatPanel.ChatInputBox` _wb_chatpanel)))
      (:`else`))))

(event `SR_SubmitChat`
  (params (PlayerName :type Text) (ChatMessage :type Text) (PlayerState :type "/Game/Network/0325/Blueprint/BP_PS_Chat Object Reference"))
  (for _array_element (`GameStateBase.PlayerArray` (`GameplayStatics.GetGameState`))
    (bind _asbp_pc_chat (cast `/Network/0325/Blueprint/BP_PC_Chat` (`PlayerState.GetPlayerController` _array_element)))
    (`self.OC_UpdateChat` _asbp_pc_chat PlayerName ChatMessage)
    (`self.TGM_CheckGoal` _asbp_pc_chat ChatMessage PlayerName PlayerState)))

(event `OC_UpdateChat`
  (params (PlayerName :type Text) (ChatMessage :type Text))
  (bind _wb_chatpanel (`self.WB_ChatPanel`)
    (:`then`
      (`/Game/Network/0325/Widget/WB_ChatPanel.Update_Chat` _wb_chatpanel PlayerName ChatMessage))
    (:`else`)))

(event `TGM_CheckGoal`
  (params (ChatMessage :type Text) (`Player Name` :type Text) (PlayerState :type "/Game/Network/0325/Blueprint/BP_PS_Chat Object Reference"))
  (bind _asbp_gm_chat (cast `/Game/Network/0325/Blueprint/BP_GM_Chat` (`GameplayStatics.GetGameMode`)))
  (`/Game/Network/0325/Blueprint/BP_GM_Chat.GetMessage` _asbp_gm_chat ChatMessage `Player Name` PlayerState))

(fn `UserConstructionScript`)