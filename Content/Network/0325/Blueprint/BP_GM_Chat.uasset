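; Game mode for a chat-based number baseball game where players guess a secret three-digit number.
; PostLogin names each player on its player state, and BeginPlay builds the random answer.
; GetMessage validates chat guesses, spends one of three chances, and prints strikes, balls and outs.
; Three strikes resets the round, as does a draw when exactly two players have exhausted their guesses, detected upon a further attempt.
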(event `self.K2_PostLogin`
  (params (NewPlayer :type "PlayerController Object Reference"))
  (bind _asbp_pc_chat (cast `/Game/Network/0325/Blueprint/BP_PC_Chat` NewPlayer))
  (bind _output_get (set `self.PC_Chat` _asbp_pc_chat))
  (bind _returnvalue (`KismetArrayLibrary.Array_Add` (`self.PlayerController`) _output_get))
  (bind _playerstate (`Controller.PlayerState` (`self.PC_Chat`))
    (:`then`
      (bind _asbp_ps_chat (cast `/Game/Network/0325/Blueprint/BP_PS_Chat` _playerstate))
      (bind _output_get_2 (set `self.PS_Chat` _asbp_ps_chat))
      (set `BSPS.PlayerNameString` (`KismetStringLibrary.Concat_StrStr` "Player " (`KismetStringLibrary.Conv_IntToString` _returnvalue)) _output_get_2))
    (:`else`)))

(event `self.ReceiveBeginPlay`
  (bind _output_get (set `self.Score` (`BaseBallScoreGenerator.GenerateRandomNumber`)))
  (for _array_element _output_get
    (set `self.GoalScore` (`KismetStringLibrary.Concat_StrStr` (`self.GoalScore`) (`KismetStringLibrary.Conv_IntToString` _array_element)))
    (`KismetSystemLibrary.PrintString` "Welcome to BaseBall Game! You need to guess 3 diffrent numbers. U have 3 chance to guess it! If u want try guess answer, chat / 3 numbers. ex) /123" true true (struct :`R` 0.96875 :`G` 1.0 :`B` 1.0 :`A` 1.0) 9999.0)))

(event `GetMessage`
  (params (GetMsg :type Text) (UsrName :type Text) (PlayerState :type "/Game/Network/0325/Blueprint/BP_PS_Chat Object Reference"))
  (set `self.UserName` UsrName)
  (bind _output_get (set `self.InComeMessage` (`KismetTextLibrary.Conv_TextToString` GetMsg)))
  (bind _returnvalue (`BaseBallCheck.CheckString` _output_get))
  (if _returnvalue
    (`KismetSystemLibrary.PrintString` (`self.GoalScore`) true true (struct :`R` 1.0 :`G` 0.0452 :`A` 1.0) 1.0)
    (`self.IncreaseGuessCount` PlayerState)
    (if (`self.HasChance`)
      (bind _returnvalue_2 (`BaseBallCheck.CheckScore` (`self.GoalScore`) (`self.InComeMessage`)))
      (bind (_strike _ball _out) (break `BaseBallResult` _returnvalue_2))
      (for (_array_element _array_index) (`|MakeArray` _strike _ball _out)
        (`|ExecutionSequence`
          (:`then_0`
            (if (== _array_index 0)
              (`KismetSystemLibrary.PrintString` (`KismetStringLibrary.Concat_StrStr` (`KismetStringLibrary.Conv_IntToString` _array_element) " Strikes!") true true (struct :`G` 0.66 :`B` 1.0 :`A` 1.0) 5.0)
              (if (== _array_element 3)
                (`KismetSystemLibrary.PrintString` (`KismetStringLibrary.Concat_StrStr` "Game Over!" (`KismetTextLibrary.Conv_TextToString` (`self.UserName`)) " Is Win!!") true true (struct :`G` 0.14433 :`B` 1.0 :`A` 1.0) 50.0)
                (`self.ResetGame`)
                (`KismetSystemLibrary.PrintString` "We got Winner! Restart Game!" true true (struct :`R` 0.418137 :`B` 1.0 :`A` 1.0) 10.0))))
          (:`then_1`
            (if (== _array_index 1)
              (`KismetSystemLibrary.PrintString` (`KismetStringLibrary.Concat_StrStr` (`KismetStringLibrary.Conv_IntToString` _array_element) " Ball!") true true (struct :`G` 0.66 :`B` 1.0 :`A` 1.0) 5.0)))
          (:`then_2`
            (if (== _array_index 2)
              (`KismetSystemLibrary.PrintString` (`KismetStringLibrary.Concat_StrStr` (`KismetStringLibrary.Conv_IntToString` _array_element) " Out!") true true (struct :`G` 0.66 :`B` 1.0 :`A` 1.0) 5.0))))))))

(event `ResetGame`
  (set `self.GoalScore` "")
  (bind _output_get (set `self.Score` (`BaseBallScoreGenerator.GenerateRandomNumber`)))
  (for _array_element _output_get
    (set `self.GoalScore` (`KismetStringLibrary.Concat_StrStr` (`self.GoalScore`) (`KismetStringLibrary.Conv_IntToString` _array_element)))
    (bind _outactors (`GameplayStatics.GetAllActorsOfClass` "/Game/Network/0325/Blueprint/BP_PS_Chat.BP_PS_Chat_C"))
    (for _array_element_2 _outactors
      (set `BSPS.CurrentGuessCount` 0 _array_element_2))))

(fn `IncreaseGuessCount`
  (params (PlayerState :type "/Game/Network/0325/Blueprint/BP_PS_Chat Object Reference"))
  (locals (PS_Chat_Local :type "/Game/Network/0325/Blueprint/BP_PS_Chat Object Reference") (MaxCounts :type Integer))
  (bind _ps_chat_local (`local.PS_Chat_Local`))
  (set `local.PS_Chat_Local` PlayerState)
  (set `self.HasChance` false)
  (if (< (`BSPS.CurrentGuessCount` (`local.PS_Chat_Local`)) 3)
    (bind _result (`/Engine/EditorBlueprintResources/StandardMacros.IncrementInt` (`BSPS.CurrentGuessCount` _ps_chat_local))
      (:`  `
        (bind _output_get (set `BSPS.CurrentGuessCount` _result _ps_chat_local))
        (`KismetSystemLibrary.PrintString` (`KismetStringLibrary.Concat_StrStr` (`BSPS.PlayerNameString` _ps_chat_local) " Left Chance : " (`KismetStringLibrary.Conv_IntToString` (- 3 _output_get))))
        (set `self.HasChance` true)))
    (else
      (`KismetSystemLibrary.PrintString` "U Lost ur Chance!")
      (bind _outactors (`GameplayStatics.GetAllActorsOfClass` "/Game/Network/0325/Blueprint/BP_PS_Chat.BP_PS_Chat_C"))
      (for _array_element _outactors
        (if (== (`BSPS.CurrentGuessCount` _array_element) 3)
          (`/Engine/EditorBlueprintResources/StandardMacros.IncrementInt` (`local.MaxCounts`))))
      (if (== (`local.MaxCounts`) 2)
        (`self.ResetGame`)
        (`KismetSystemLibrary.PrintString` "We are Draw.... Restart Game!" true true (struct :`R` 0.857666 :`B` 1.0 :`A` 1.0) 10.0)
        (else
          (set `local.MaxCounts` 0))))))

(fn `UserConstructionScript`)