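; Actor component that provides in-game text chat, creating the chat widget for a local baseball player controller and binding its send-message event.
; Enter focuses the chat box and the mouse wheel scrolls it.
; SendChatMessageOnServer loops over the PlayerArray, calling each controller's chat component to add the message to that player's chat box.
; Separate events forward messages to the baseball GameMode or print broadcasts on authority.
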(event `self.ReceiveBeginPlay`
  (if (`Controller.IsLocalPlayerController` (cast `/Game/Network/Blueprint/BP_BaseBallPlayerController` (`self.GetOwner`) :!pure true))
    (bind _returnvalue (`|CreateWidget` "/Game/Network/Blueprint/NBC/UMG_ChatUI.UMG_ChatUI_C"))
    (bind _output_get (set `self.ChatUI_Ref` _returnvalue))
    (`UserWidget.AddToViewport` _output_get 0)
    (set `self.ChatBoxRef` (`/Game/Network/Blueprint/NBC/UMG_ChatUI.UMG_ChatWindow` _output_get))
    (add `/Game/Network/Blueprint/NBC/UMG_ChatWindow.SetMessageToUserController` (`self.ChatBoxRef`) (`|CreateDelegate` :!event `OnSendMsgToServer`))))

(event `Key|Enter`
  (params (Key :type "Key Structure"))
  (:`Pressed`
    (`/Game/Network/Blueprint/NBC/UMG_ChatWindow.Focus Chat` (`self.ChatBoxRef`))))

(event `Key|MouseScrollUp`
  (params (Key :type "Key Structure"))
  (:`Pressed`
    (`/Game/Network/Blueprint/NBC/UMG_ChatWindow.Scroll` (`self.ChatBoxRef`) true)))

(event `Key|MouseScrollDown`
  (params (Key :type "Key Structure"))
  (:`Pressed`
    (`/Game/Network/Blueprint/NBC/UMG_ChatWindow.Scroll` (`self.ChatBoxRef`) false)))

(event `GotBroadCast`
  (params (Msg :type String))
  (if (`Actor.HasAuthority` (`self.GetOwner`))
    (`KismetSystemLibrary.PrintString` Msg true true (struct :`G` 0.66 :`B` 1.0 :`A` 1.0) 10.0)))

(event `SendChatMessageOnServer`
  (params (Message :type String) (UserName :type String))
  (for _array_element (`GameStateBase.PlayerArray` (`GameplayStatics.GetGameState`))
    (`self.AddChatMessageOnOwningClient` (`Actor.GetComponentByClass` (`PlayerState.GetPlayerController` _array_element) "BP_NBCChatActorComponent_C") Message (`self.User ID`))))

(event `AddChatMessageOnOwningClient`
  (params (Message :type String) (`Player Name` :type String))
  (`/Game/Network/Blueprint/NBC/UMG_ChatWindow.AddChatMessage` (`self.ChatBoxRef`) Message `Player Name`))

(event `OnSendMsgToServer`
  (params (Msg :type String))
  (bind _asbp_base_ball_game_mode_base (cast `/Game/Network/Blueprint/BP_BaseBallGameModeBase` (`GameplayStatics.GetGameMode`)))
  (`/Game/Network/Blueprint/BP_BaseBallGameModeBase.GotMessageFromClient` _asbp_base_ball_game_mode_base Msg (`self.PlayerState`)))